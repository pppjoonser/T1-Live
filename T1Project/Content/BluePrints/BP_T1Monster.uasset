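; BP_T1Monster is an AI-controlled enemy monster whose death reports a true game result to BP_T1GameMode.
; CombatSystem HP events are bound at BeginPlay, and UpdateHp feeds the overhead HP bar widget.
; Attack turns toward the target, sets the AnimBP flag and disables movement until a timer ends it, while AttackHitCheck sphere-traces forward to deal damage.
; SetDead plays the death montage, hides the bar, disables collision and stops the AI.
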(event `self.ReceiveBeginPlay`
  (add `/Game/CombatComponent.OnChangeHp` (`self.CombatSystem`) (`|CreateDelegate` :!event `UpdateHp`))
  (add `/Game/CombatComponent.OnHpZero` (`self.CombatSystem`) (`|CreateDelegate` :!event `SetDead`))
  (cast `/Game/UI/WBP_HpBar` (`WidgetComponent.GetUserWidgetObject` (`self.HpBarComponent`)))
  (`self.UpdateHp` (`/Game/CombatComponent.Hp` (`self.CombatSystem`)) (`/Game/CombatComponent.MaxHp` (`self.CombatSystem`))))

(fn `Attack`
  (params (TargetActor :type "Actor Object Reference"))
  (bind (_returnvalue_roll _returnvalue_pitch _returnvalue_yaw) (`KismetMathLibrary.BreakRotator` (`KismetMathLibrary.FindLookAtRotation` (`self.K2_GetActorLocation`) (`self.K2_GetActorLocation` TargetActor))))
  (`/Engine/EditorBlueprintResources/StandardMacros.IsValid` TargetActor
    (:`Is Valid`
      (`self.K2_SetActorRotation` (`KismetMathLibrary.MakeRotator` 0.0 0.0 _returnvalue_yaw))
      (bind _asabp_t1monster (cast `/Game/Animation/ABP_T1Monster` (`SkeletalMeshComponent.GetAnimInstance` (`self.Mesh`))))
      (set `/Game/Animation/ABP_T1Monster.bAttack` true _asabp_t1monster)
      (`KismetSystemLibrary.K2_SetTimer` null "AttackEnded" 1.0)
      (`CharacterMovementComponent.SetMovementMode` (`self.CharacterMovement`) "MOVE_None" 0))))

(fn `AttackEnded`
  (bind _asabp_t1monster (cast `/Game/Animation/ABP_T1Monster` (`SkeletalMeshComponent.GetAnimInstance` (`self.Mesh`))))
  (set `/Game/Animation/ABP_T1Monster.bAttack` false _asabp_t1monster)
  (`CharacterMovementComponent.SetMovementMode` (`self.CharacterMovement`) "MOVE_Walking" 0))

(fn `AttackHitCheck`
  (bind _returnvalue (`self.K2_GetActorLocation`))
  (bind (_outhit _returnvalue_2) (`KismetSystemLibrary.SphereTraceSingle` :`Start` _returnvalue :`End` (+ _returnvalue (* (`self.GetActorForwardVector`) (`self.AttackRange`))) :`Radius` (`self.AttackRadius`) :`TraceChannel` "TraceTypeQuery4" :`DrawDebugType` "ForDuration" :`DrawTime` 0.5))
  (if _returnvalue_2
    (`/Game/CombatComponent.CombatAttack` (`self.CombatSystem`) (`self.AttackDamage`) (`.HitActor` (`GameplayStatics.BreakHitResult` _outhit)))))

(fn `SetDead`
  (`self.PlayAnimMontage` "/Game/Animation/AM_MonsterDeath.AM_MonsterDeath")
  (`SceneComponent.SetHiddenInGame` (`self.HpBarComponent`) true false)
  (`self.SetActorEnableCollision` false)
  (bind _asbp_t1monster_controller (cast `/Game/BluePrints/BP_T1MonsterController` (`self.GetController`)))
  (`/Game/BluePrints/BP_T1MonsterController.StopAI` _asbp_t1monster_controller)
  (bind _asbp_t1game_mode (cast `/Game/BluePrints/BP_T1GameMode` (`GameplayStatics.GetGameMode`)))
  (`/Game/BluePrints/BP_T1GameMode.GameResult` _asbp_t1game_mode true))

(fn `UpdateHp`
  (params (NewHp :type "Float (double-precision)") (NewMaxHp :type "Float (double-precision)"))
  (bind _aswbp_hp_bar (cast `/Game/UI/WBP_HpBar` (`WidgetComponent.GetUserWidgetObject` (`self.HpBarComponent`))))
  (`/Game/UI/WBP_HpBar.UpdateHpBar` _aswbp_hp_bar NewHp NewMaxHp))

(fn `UserConstructionScript`)